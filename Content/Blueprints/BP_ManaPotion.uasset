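; BP_ManaPotion is a pickup potion the player can hold, drop or use.
; Overlapping its trigger asks BP_ThirdPersonCharacter_Custom to pick it up; Pickup snaps it to the hand_l socket and disables trigger collision.
; Drop detaches it, enables physics and collision with gravity off, then destroys it after a short delay.
; PrimaryAction only prints a mana gain message and destroys the potion, without changing any mana value.
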(event `self.PickupTrigger.OnComponentBeginOverlap`
  (params (OverlappedComponent :type "PrimitiveComponent Object Reference") (OtherActor :type "Actor Object Reference") (OtherComp :type "PrimitiveComponent Object Reference") (OtherBodyIndex :type Integer) (bFromSweep :type Boolean) (SweepResult :type "HitResult Structure (by ref)"))
  (bind _asbp_third_person_character_custom (cast `/Game/Blueprints/BP_ThirdPersonCharacter_Custom` OtherActor))
  (`/Game/Blueprints/BP_ThirdPersonCharacter_Custom.TryToPickUp` _asbp_third_person_character_custom self))

(event `self.Pickup`
  (params (ParentMesh :type "SkeletalMeshComponent Object Reference"))
  (`SceneComponent.K2_AttachToComponent` (`self.DefaultSceneRoot`) ParentMesh "hand_l" "SnapToTarget" "SnapToTarget" "KeepRelative" true)
  (`PrimitiveComponent.SetCollisionEnabled` (`self.PickupTrigger`) "NoCollision"))

(event `self.Drop`
  (`SceneComponent.K2_DetachFromComponent` (`self.DefaultSceneRoot`) "KeepWorld" "KeepWorld" "KeepWorld" true) ; Leaves the hand
  (`PrimitiveComponent.SetSimulatePhysics` (`self.PickupTrigger`) true)
  (`PrimitiveComponent.SetSimulatePhysics` (`self.Mana_Potion`) true) ; Turns physics on
  (`PrimitiveComponent.SetCollisionEnabled` (`self.Mana_Potion`) "QueryAndPhysics") ; Turns collision on
  (`PrimitiveComponent.SetEnableGravity` (`self.Mana_Potion`) false)
  (`KismetSystemLibrary.Delay` 2.0)
  (`self.K2_DestroyActor`))

(event `self.PrimaryAction`
  (`KismetSystemLibrary.PrintString` "Plus 10 mana!")
  (`self.K2_DestroyActor`))

(fn `UserConstructionScript`)