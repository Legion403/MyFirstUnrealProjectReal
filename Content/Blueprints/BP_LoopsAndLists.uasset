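; BP_LoopsAndLists is an Actor Blueprint that demonstrates loop and array techniques by printing messages to the screen.
; BeginPlay enables input and starts two delay-based loops: a self-calling event that stops after a counter limit and an endless once-per-second wire loop.
; An input action runs a while loop within one frame, printing in random colors, then resets its counter.
; Number keys print a hardcoded name array's length or list its entries.
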(event `Recursive Loop`
  (if (> (`self.RecursionCounter`) 4)
    (`KismetSystemLibrary.PrintString` "Looped 5 times")
    (else
      (bind _result (`/Engine/EditorBlueprintResources/StandardMacros.IncrementInt` (`self.RecursionCounter`)) ; Adds 1 to recursion counter
        (:`  `
          (`KismetSystemLibrary.PrintString` (`KismetStringLibrary.Concat_StrStr` "The Recursive loop has run " (`KismetStringLibrary.Conv_IntToString` _result)) true true (struct :`G` 0.66 :`B` 1.0 :`A` 1.0) 1.3)
          (`KismetSystemLibrary.Delay` 2.0)
          (`self.Recursive Loop`) ; Calling the event to start it all over
        )))))

(event `InputAction|Start While Loop`
  (params (Key :type "Key Structure"))
  (bind _whileloopcounter (`self.WhileLoopCounter`))
  (:`Pressed`
    (`KismetSystemLibrary.PrintString` "Starting While Loop!")
    ; While Loops Body
    (while (< (`self.WhileLoopCounter`) 25)
      (`/Engine/EditorBlueprintResources/StandardMacros.IncrementInt` _whileloopcounter
        (:`  `
          (`KismetSystemLibrary.PrintString` (`KismetStringLibrary.Concat_StrStr` "This While Loop Has Run " (`KismetStringLibrary.Conv_IntToString` _whileloopcounter) "Times!") true true (`KismetMathLibrary.MakeColor` (`KismetMathLibrary.RandomFloat`) (`KismetMathLibrary.RandomFloat`) (`KismetMathLibrary.RandomFloat`))))))
    (`KismetSystemLibrary.PrintString` "While Loop Is Done!")
    (set `self.WhileLoopCounter` 0)))

(event `self.ReceiveBeginPlay`
  (`self.Recursive Loop`)
  (`KismetSystemLibrary.PrintString` "Loops and lists is startin g")
  (`self.Simple game loop`)
  (`self.EnableInput` (`GameplayStatics.GetPlayerController` 0)))

(event `Simple game loop`
  (`KismetSystemLibrary.PrintString` "Starting Game Loop" true true (struct :`R` 1.0 :`G` 0.030437 :`B` 0.878482 :`A` 1.0) 0.6 :!label _label) ; Print a string
  (`KismetSystemLibrary.Delay` 1.0) ; Wait a sec
  (goto _label))

(event `Key|Six`
  (params (Key :type "Key Structure"))
  (:`Pressed`
    (`self.First Array Test`)))

(event `First Array Test`
  (`KismetSystemLibrary.PrintString` (`KismetStringLibrary.Concat_StrStr` "Our array of names is" (`KismetStringLibrary.Conv_IntToString` (`KismetArrayLibrary.Array_Length` (`|MakeArray` "Lea" "Luke" "Han" "Chewey" "Anakin" "Threepeo"))) "Names long")))

(event `List all names`
  (for (_array_element _array_index) (`|MakeArray` "Lea" "Luke" "Han" "Chewey" "Anakin" "Threepeo")
    (`KismetSystemLibrary.PrintString` (`KismetStringLibrary.Concat_StrStr` (`KismetStringLibrary.Conv_IntToString` (+ _array_index 1)) _array_element))))

(event `Key|Five`
  (params (Key :type "Key Structure"))
  (:`Pressed`
    (`self.List all names`)))

(fn `UserConstructionScript`)