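; BP_BasicEnemy is a simple enemy that swings a sword and dies when the player overlaps its capsule.
; A looping Timeline lerps the sword's rotation, pausing between swings.
; Sword overlaps with any actor raise a hit counter; past the threshold, a player overlap loads the checkpoint and resets the count.
; On death, the cylinder simulates physics, then after a delay Manager checks the enemy count and the actor is destroyed.
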(event `self.ReceiveBeginPlay`
  (`self.Swing Sword`))

(event `self.Capsule.OnComponentBeginOverlap`
  (params (OverlappedComponent :type "PrimitiveComponent Object Reference") (OtherActor :type "Actor Object Reference") (OtherComp :type "PrimitiveComponent Object Reference") (OtherBodyIndex :type Integer) (bFromSweep :type Boolean) (SweepResult :type "HitResult Structure (by ref)"))
  (cast `/Game/Blueprints/BP_ThirdPersonCharacter_Custom` OtherActor)
  (`PrimitiveComponent.SetSimulatePhysics` (`self.Cylinder`) true)
  (`KismetSystemLibrary.Delay` 2.5)
  (`/Game/Blueprints/Enemies/BP_EnemySpawnManager.Check Enemy Count` (`self.Manager`))
  (`self.K2_DestroyActor`))

(event `self.Sword_For_Prototype.OnComponentBeginOverlap`
  (params (OverlappedComponent :type "PrimitiveComponent Object Reference") (OtherActor :type "Actor Object Reference") (OtherComp :type "PrimitiveComponent Object Reference") (OtherBodyIndex :type Integer) (bFromSweep :type Boolean) (SweepResult :type "HitResult Structure (by ref)"))
  (if (> (`self.Hits`) 1)
    (bind _asbp_third_person_character_custom (cast `/Game/Blueprints/BP_ThirdPersonCharacter_Custom` OtherActor))
    (`/Game/Blueprints/BP_ThirdPersonCharacter_Custom.Load Checkpoint` _asbp_third_person_character_custom)
    (`KismetSystemLibrary.PrintString` "Ouch!")
    (set `self.Hits` 0)
    (else
      (`/Engine/EditorBlueprintResources/StandardMacros.IncrementInt` (`self.Hits`)))))

(event `Swing Sword`
  (bind (_direction _newtrack_0) (`Timeline|Timeline` :!label _label)
    (:`Update`
      (`SceneComponent.K2_SetWorldRotation` (`self.Sword_For_Prototype`) (`KismetMathLibrary.RLerp` (struct :`Yaw` -37.0) (struct :`Yaw` 43.0) _newtrack_0) false false))
    (:`Finished`
      (`KismetSystemLibrary.Delay` 2.0)
      (goto _label :!via `PlayFromStart`))))

(fn `UserConstructionScript`)