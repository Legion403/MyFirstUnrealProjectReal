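; Enemy wave manager that spawns a BP_BasicEnemy at every BP_EnemySpawner in the level.
; On BeginPlay it caches all spawners, then spawns one enemy at each, passing itself as that enemy's Manager and counting it.
; CheckEnemyCount decrements the live total and, when none remain, waits briefly, announces a new wave and respawns at all spawners.
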(event `self.ReceiveBeginPlay`
  (`KismetSystemLibrary.PrintString` "Enemy Spawn manager is ready")
  (bind _outactors (`GameplayStatics.GetAllActorsOfClass` "/Game/Blueprints/Enemies/BP_EnemySpawner.BP_EnemySpawner_C"))
  (set `self.Spawners` _outactors)
  (`self.Spawn Enemies`))

(event `Spawn Enemies`
  (for _array_element (`self.Spawners`)
    (bind (_returnvalue_location _returnvalue_rotation) (`KismetMathLibrary.BreakTransform` (`SceneComponent.K2_GetComponentToWorld` (`/Game/Blueprints/Enemies/BP_EnemySpawner.DefaultSceneRoot` _array_element))))
    (bind _returnvalue (`|SpawnActorFromClass` "/Game/Blueprints/Enemies/BP_BasicEnemy.BP_BasicEnemy_C" (`KismetMathLibrary.MakeTransform` _returnvalue_location _returnvalue_rotation) "AdjustIfPossibleButAlwaysSpawn" "MultiplyWithRoot" null null)) ; Create a new enemy At spawner location
    (set `/Game/Blueprints/Enemies/BP_BasicEnemy.Manager` self _returnvalue) ; Assign this manager to the manager variable on each enemy
    (`/Engine/EditorBlueprintResources/StandardMacros.IncrementInt` (`self.CurrentEnemyTotal`))))

(event `Check Enemy Count`
  (`/Engine/EditorBlueprintResources/StandardMacros.DecrementInt` (`self.CurrentEnemyTotal`)
    (:`  `
      (if (not (> (`self.CurrentEnemyTotal`) 0))
        (`KismetSystemLibrary.Delay` 2.0)
        (`KismetSystemLibrary.PrintString` "NEW WAVE INCOMING!!!")
        (`self.Spawn Enemies`)))))

(fn `UserConstructionScript`)