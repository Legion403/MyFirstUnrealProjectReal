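; BP_Key is a collectible key pickup that increments the player's key count.
; On BeginPlay it converts a random integer to the KeyColors enum and switches on it to apply one of several materials to the cube mesh.
; When BP_ThirdPersonCharacter_Custom overlaps its box, the key adds one to that character's KeyCount, prints debug messages with the new total, and destroys itself.
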(event `self.ReceiveBeginPlay`
  (switch `/Game/Blueprints/KeyColors` (cast `/Game/Blueprints/KeyColors` (`KismetMathLibrary.Conv_IntToByte` (`KismetMathLibrary.RandomIntegerInRange` 1 5))) ; Changes depending on the random number
    (:`NewEnumerator0`
      (`PrimitiveComponent.SetMaterial` (`self.cube_0`) 0 "/Game/StarterContent/Materials/M_Metal_Burnished_Steel.M_Metal_Burnished_Steel"))
    (:`NewEnumerator1`
      (`PrimitiveComponent.SetMaterial` (`self.cube_0`) 0 "/Game/StarterContent/Materials/M_Metal_Gold.M_Metal_Gold"))
    (:`NewEnumerator2`
      (`PrimitiveComponent.SetMaterial` (`self.cube_0`) 0 "/Game/StarterContent/Materials/M_Tech_Hex_Tile_Pulse.M_Tech_Hex_Tile_Pulse"))
    (:`NewEnumerator3`
      (`PrimitiveComponent.SetMaterial` (`self.cube_0`) 0 "/Game/StarterContent/Props/Materials/M_Frame.M_Frame"))
    (:`NewEnumerator4`
      (`PrimitiveComponent.SetMaterial` (`self.cube_0`) 0 "/Game/LevelPrototyping/Interactable/JumpPad/Assets/Materials/M_GradientGlow.M_GradientGlow"))))

(event `self.Box.OnComponentBeginOverlap`
  (params (OverlappedComponent :type "PrimitiveComponent Object Reference") (OtherActor :type "Actor Object Reference") (OtherComp :type "PrimitiveComponent Object Reference") (OtherBodyIndex :type Integer) (bFromSweep :type Boolean) (SweepResult :type "HitResult Structure (by ref)"))
  (bind _asbp_third_person_character_custom (cast `/Game/Blueprints/BP_ThirdPersonCharacter_Custom` OtherActor))
  (`KismetSystemLibrary.PrintString` "A player ran into me!" true true (struct :`G` 0.66 :`B` 1.0 :`A` 1.0) 6.0)
  (bind _keycount (`/Game/Blueprints/BP_ThirdPersonCharacter_Custom.KeyCount` _asbp_third_person_character_custom))
  (set `/Game/Blueprints/BP_ThirdPersonCharacter_Custom.KeyCount` (+ _keycount 1) _asbp_third_person_character_custom)
  (`KismetSystemLibrary.PrintString` (`KismetStringLibrary.Concat_StrStr` "The player has " (`KismetStringLibrary.Conv_IntToString` _keycount) " keys!"))
  (`self.K2_DestroyActor`))

(fn `UserConstructionScript`)