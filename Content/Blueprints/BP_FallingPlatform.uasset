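; BP_FallingPlatform is a platform that drops shortly after the custom third-person character overlaps its collision box, then returns to its start.
; Activate waits briefly, sets the activated flag and a material, then Drop enables physics simulation on the mesh.
; After another delay, Reset disables physics and a timeline lerps the mesh back to the transform saved at BeginPlay, clearing the flag when finished.
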(event `self.ReceiveBeginPlay`
  (set `self.StartingTransform` (`SceneComponent.K2_GetComponentToWorld` (`self.Falling_Platform_No_Animation`))) ; SAving starter location of the platform
)

(event `self.PlatCollision.OnComponentBeginOverlap`
  (params (OverlappedComponent :type "PrimitiveComponent Object Reference") (OtherActor :type "Actor Object Reference") (OtherComp :type "PrimitiveComponent Object Reference") (OtherBodyIndex :type Integer) (bFromSweep :type Boolean) (SweepResult :type "HitResult Structure (by ref)"))
  (cast `/Game/Blueprints/BP_ThirdPersonCharacter_Custom` OtherActor) ; Did the player hit the collision box
  (`self.Activate`))

(event `Activate`
  (if (not (`self.IsActivated`))
    (`KismetSystemLibrary.PrintString` "ONE SECOND LEFT!!!")
    (`KismetSystemLibrary.Delay` 1.0)
    (set `self.IsActivated` true)
    (`PrimitiveComponent.SetMaterial` (`self.Falling_Platform_No_Animation`) 0 "/Game/Characters/Moving_Platform/Materials/Material_001.Material_001")
    (`self.Drop`)))

(event `Drop`
  (if (`self.IsActivated`)
    (`KismetSystemLibrary.PrintString` "Dropping!")
    (`PrimitiveComponent.SetSimulatePhysics` (`self.Falling_Platform_No_Animation`) true)
    (`KismetSystemLibrary.Delay` 3.0)
    (`PrimitiveComponent.SetMaterial` (`self.Falling_Platform_No_Animation`) 0 "/Game/Characters/Falling_Platform/Materials/Material_001.Material_001")
    (`self.Reset`)))

(event `Reset`
  (`KismetSystemLibrary.PrintString` "Reseting!")
  (set `self.ResetTransform` (`SceneComponent.K2_GetComponentToWorld` (`self.Falling_Platform_No_Animation`)))
  (`PrimitiveComponent.SetSimulatePhysics` (`self.Falling_Platform_No_Animation`) false) ; turns physics back off
  (bind (_direction _newtrack_0) (`Timeline|TimelineForFP`)
    (:`Update`
      (bind (_returnvalue_location _returnvalue_rotation) (`KismetMathLibrary.BreakTransform` (`KismetMathLibrary.TLerp` (`self.ResetTransform`) (`self.StartingTransform`) _newtrack_0)))
      (`SceneComponent.K2_SetWorldLocationAndRotation` (`self.Falling_Platform_No_Animation`) _returnvalue_location _returnvalue_rotation false false))
    (:`Finished`
      (set `self.IsActivated` false))))

(fn `UserConstructionScript`)